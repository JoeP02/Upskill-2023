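; BP_ShooterPlayerController is a player controller that toggles the pause menu in a shooter.
; The Pause input action checks the paused state, then either pauses and adds a new WBP_Pause widget to the viewport, or unpauses and removes it.
; Each toggle also switches input between Game And UI, focused on the widget, and Game Only, showing or hiding the mouse cursor to match.
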(event EventBeginPlay)

(event EventTick
  (params (DeltaSeconds :type Float%20%28single-precision%29)))

(event Input|ActionEvents|InputActionPause
  (params (Key :type Key%20Structure :default "None"))
  (bind _returnvalue (Game|GetPlayerController 0))
  (:Pressed
    (if (Game|IsGamePaused)
      (Game|SetGamePaused false)
      (Widget|RemovefromParent (stale _returnvalue_2))
      (Input|SetInputModeGameOnly _returnvalue)
      (Variables|/Script/Engine.PlayerController|SetbShowMouseCursor _returnvalue false)
      (else
        (Game|SetGamePaused true)
        (bind _returnvalue_2 (UserInterface|CreateWidget "/Game/UI/WBP_Pause.WBP_Pause_C"))
        (UserInterface|Viewport|AddtoViewport _returnvalue_2 0)
        (Input|SetInputModeGameandUI _returnvalue _returnvalue_2 "DoNotLock" true)
        (Variables|/Script/Engine.PlayerController|SetbShowMouseCursor _returnvalue true)))))

(fn ConstructionScript)